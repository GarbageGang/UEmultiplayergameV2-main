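; Game instance Blueprint that shows the join game menu as the main menu through a single UI function.
; It creates the WB_JoinGameMenu widget for the first player controller only when the cached reference is invalid, then adds it to the viewport.
; It switches that controller to UI-only input with a visible cursor, taking the focus target from the creation output rather than the cached reference.
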(fn `UI_ShowMainMenu`
  (bind _returnvalue (`GameplayStatics.GetPlayerController` 0))
  (`/Engine/EditorBlueprintResources/StandardMacros.IsValid` (`self.WB`)
    (:`Is Valid`
      _)
    (:`Is Not Valid`
      (bind _returnvalue_2 (`|CreateWidget` "/Game/Widgets/WB_JoinGameMenu.WB_JoinGameMenu_C" (`GameplayStatics.GetPlayerController` 0)))
      (set `self.WB` _returnvalue_2)))
  (`UserWidget.AddToViewport` (`self.WB`) 0)
  (`WidgetBlueprintLibrary.SetInputMode_UIOnlyEx` _returnvalue _returnvalue_2)
  (set `PlayerController.bShowMouseCursor` true _returnvalue)
  (return))