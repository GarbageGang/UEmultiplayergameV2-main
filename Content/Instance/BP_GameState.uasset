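; Game state Blueprint that runs a server-authoritative countdown shared through the replicated Time variable.
; On BeginPlay, the authority starts a looping one-second timer that decrements Time, with no stop condition in the graph.
; OnRep_Time passes each new value to the OnTimerUpdate event dispatcher, so listeners react to changes without polling.
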(event `self.ReceiveBeginPlay`
  (`self.StartTimer`))

(event `StartTimer`
  (`/Engine/EditorBlueprintResources/ActorMacros.Switch Has Authority`
    (:`Authority`
      (`KismetSystemLibrary.K2_SetTimerDelegate` (delegate `TimerDecrement`) 1.0 true)
      (`KismetSystemLibrary.PrintText` "Timer Created"))))

(event `TimerDecrement`
  (`/Engine/EditorBlueprintResources/StandardMacros.DecrementFloat` (`self.Time`)))

(fn `OnRep_Time`
  (`self.OnTimerUpdate` (`self.Time`)))

(fn `UserConstructionScript`)