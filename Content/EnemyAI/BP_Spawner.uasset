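; Server-authoritative enemy spawner actor that periodically populates the area around itself with AI enemies.
; On BeginPlay, a looping timer is set only on the authority, firing the spawn event at a fixed interval.
; Each tick of that timer, while the enemy count is below its cap, it increments the count and spawns BP_Enemy with its behavior tree at a random navigable point within a radius.
; The count never decreases here.
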(event `self.ReceiveBeginPlay`
  (`self.ServerSpawn`))

(event `ServerSpawn`
  (`/Engine/EditorBlueprintResources/ActorMacros.Switch Has Authority`
    (:`Authority`
      (`KismetSystemLibrary.K2_SetTimerDelegate` (delegate `SpawnEnemy`) 10.0 true))))

(event `SpawnEnemy`
  (if (< (`self.Enemies`) (`self.MaxEnemies`))
    (`/Engine/EditorBlueprintResources/StandardMacros.IncrementInt` (`self.Enemies`)
      (:`  `
        (bind _randomlocation (`NavigationSystemV1.K2_GetRandomLocationInNavigableRadius` (`self.K2_GetActorLocation`) (`self.MaxRadius`) null null))
        (`AIBlueprintHelperLibrary.SpawnAIFromClass` "/Game/ThirdPerson/Blueprints/BP_Enemy.BP_Enemy_C" "/Game/EnemyAI/BT_EnemyAI1.BT_EnemyAI1" _randomlocation (struct) false null)
        (`KismetSystemLibrary.PrintText` "Enemy Spawned")))))

(fn `UserConstructionScript`)